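; BP_ParallaxBG is a parallax background actor that displays a configurable texture on a plane.
; Its construction script creates a dynamic instance of MI_ParallaxMat, feeds it the texture, view distance, height, center and offset variables, then applies it to the Plane.
; The Blueprint runs no gameplay logic, leaving any parallax motion to the material.
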(event EventBeginPlay)

(event Collision|EventActorBeginOverlap
  (params (OtherActor :type Actor%20Object%20Reference)))

(event EventTick
  (params (DeltaSeconds :type Float%20%28single-precision%29)))

(fn ConstructionScript
  (bind _returnvalue (Rendering|Material|CreateDynamicMaterialInstance (Variables|Default|GetPlane) 0 "/Game/PaperAssets/Custom/GrassyMountainsParallax/MI_ParallaxMat.MI_ParallaxMat" "None" :!class /Script/Engine.PrimitiveComponent))
  (Variables|Default|SetMatInst _returnvalue)
  (Rendering|Material|SetTextureParameterValue (Variables|Default|GetMatInst) "BG_Texture" (Variables|MaterialParameters|GetTexture))
  (Rendering|Material|SetScalarParameterValue (Variables|Default|GetMatInst) "BG_Distance" (Variables|Default|GetDistanceFromView) :!class /Script/Engine.MaterialInstanceDynamic)
  (Rendering|Material|SetScalarParameterValue (Variables|Default|GetMatInst) "Height" (Variables|Default|GetHeight) :!class /Script/Engine.MaterialInstanceDynamic)
  (Rendering|Material|SetVectorParameterValue (Variables|Default|GetMatInst) "BG_Center" (Variables|Default|GetCenter) :!class /Script/Engine.MaterialInstanceDynamic)
  (Rendering|Material|SetVectorParameterValue (Variables|Default|GetMatInst) "BG_Offset" (Variables|Default|GetOffset) :!class /Script/Engine.MaterialInstanceDynamic)
  (Rendering|Material|SetMaterial (Variables|Default|GetPlane) 0 (Variables|Default|GetMatInst)))